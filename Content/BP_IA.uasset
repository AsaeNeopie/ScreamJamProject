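; AI bot that wanders the level and chases pawns it sees, honking a Cucaracha klaxon when it reaches one.
; Walk loops AI MoveTo toward random reachable points around the bot, restarting on each success.
; PawnSensing sightings redirect movement to the seen pawn, and a one-second retriggerable delay resumes wandering once sightings stop.
; The horn sits behind a DoOnce that resets only if PlaySound finds PawnSensing invalid.
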(event OnSeePawn(PawnSensing)
  (params (Pawn :type Pawn%20Object%20Reference))
  ;[1 1 1] Deplacement bot
  (Utilities|FlowControl|Sequence
    (:then_0
      (AI|AIMoveTo self "0, 0, 0" Pawn 5.0 false
        (:OnSuccess
          (CallFunction|PlaySound))))
    (:then_1
      (Utilities|FlowControl|RetriggerableDelay 1.0)
      (CallFunction|Walk))))

(event Custom|Walk
  ;[1 1 1] Deplacement bot
  (AI|AIMoveTo self (.RandomLocation (AI|Navigation|GetRandomReachablePointinRadius (Transformation|GetActorLocation) 1.5e+03 0 0)) 0 5.0 false
    (:OnSuccess
      (CallFunction|Walk))))

(event Custom|PlaySound
  (Variables|Default|GetPawnSensing
    (:then
      (Utilities|FlowControl|DoOnce false :!label _label
        (:Completed
          (Audio|Components|Audio|Play (Variables|Default|GetKlaxon_cucaracha_12v) 0.0))))
    (:else
      (goto _label Reset))))

(event EventBeginPlay
  ;[1 1 1] Deplacement bot
  (CallFunction|Walk))

(fn ConstructionScript)