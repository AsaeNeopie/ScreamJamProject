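; Teleport trigger actor that moves any Pawn overlapping it, with debug print and debug point.
; With SnapOnGround, a capsule trace sized to player 0 runs upward from TPposition relative to the actor, and the pawn lands just above the hit location.
; A horizontal entry offset is added only when KeepOriginaloffset is false.
; Without SnapOnGround, the trigger actor itself, not the pawn, moves to raw TPposition.
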(event Collision|EventActorBeginOverlap
  (params (OtherActor :type Actor%20Object%20Reference))
  (bind _returnvalue (Game|GetPlayerCharacter 0))
  (bind _capsulecomponent (Variables|/Script/Engine.Character|GetCapsuleComponent _returnvalue))
  (bind _returnvalue_2 (Components|Capsule|GetScaledCapsuleHalfHeight _capsulecomponent))
  (Development|PrintString "tp")
  (bind _aspawn (Utilities|Casting|CastToPawn OtherActor))
  (if (Variables|Default|GetkeepOriginaloffset)
    (Variables|Default|Setoffset "0, 0, 0")
    (else
      (Variables|Default|Setoffset (* (- (Transformation|GetActorLocation _aspawn) (Transformation|GetActorLocation)) "1.000000,1.000000,0.000000"))))
  (if (Variables|Default|GetSnapOnGround)
    (bind _outhit (Collision|CapsuleTraceByChannel (+ (Variables|Default|GetTPposition) (Transformation|GetActorLocation) (Variables|Default|Getoffset)) (+ (+ (Variables|Default|GetTPposition) (Transformation|GetActorLocation) (Variables|Default|Getoffset)) "0.000000,0.000000,10000.000000") (Components|Capsule|GetScaledCapsuleRadius _capsulecomponent) _returnvalue_2 "TraceTypeQuery1" false 0 "None"))
    (Rendering|Debug|DrawDebugPoint (+ (* _returnvalue_2 "0.000000,0.000000,1.000000") (.Location (Collision|BreakHitResult _outhit)) "0.000000,0.000000,5.000000") 5e+01 "(R=1.000000,G=0.485138,B=0.252246,A=1.000000)" 3.0)
    (Transformation|SetActorLocation _aspawn (+ (* _returnvalue_2 "0.000000,0.000000,1.000000") (.Location (Collision|BreakHitResult _outhit)) "0.000000,0.000000,5.000000") false (Variables|Default|Getteleport))
    (else
      (Transformation|SetActorLocation (Variables|Default|GetTPposition) false (Variables|Default|Getteleport)))))

(fn ConstructionScript)